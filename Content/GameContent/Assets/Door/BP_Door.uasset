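; BP_Door is a gate that slides open once enough items have been collected.
; Each CollectedItem call increments a counter, and reaching MaxItems fires OpenDoor through a DoOnce and prints a message.
; OpenDoor plays the DoorRotation timeline, which, despite its name, lerps the relative X locations of the two door panels in opposite directions by unequal distances.
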(event Custom|Open%20Door
  (bind _door_rotation (Timeline|Door%20Rotation Play)
    (:Update
      (Transformation|SetRelativeLocation (Variables|Default|GetDoorleft) (Math|Vector|MakeVector (Math|Float|Lerp 0.0 3.5e+02 _door_rotation) 0.0 0.0) false false)
      (Transformation|SetRelativeLocation (Variables|Default|GetDoorright) (Math|Vector|MakeVector (Math|Float|Lerp 0.0 -7e+02 _door_rotation) 0.0 0.0) false false))))

(event Custom|Collected%20Item
  (Math|Integer|IncrementInt (Variables|Default|GetCurrent%20Items)
    (:%20%20
      (if (>= (Variables|Default|GetCurrent%20Items) (Variables|Default|GetMaxItems))
        (Utilities|FlowControl|DoOnce false
          (:Completed
            (CallFunction|OpenDoor)
            (Development|PrintString "The Gate Has Opened")))))))

(fn ConstructionScript)