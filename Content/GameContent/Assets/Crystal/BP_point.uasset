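; BP_point is a collectible that counts toward a door when the Shapeshifter_original character touches it.
; On sphere overlap it calls CollectedItem on the BP_Door found via GetActorOfClass, destroys itself and plays an explosion sound.
; The construction script gives its InterpToMovement two relative control points, the origin and the Pos variable, defining a movement path for each placed instance.
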(event OnComponentBeginOverlap(Sphere)
  (params (OverlappedComponent :type Primitive%20Component%20Object%20Reference) (OtherActor :type Actor%20Object%20Reference) (OtherComp :type Primitive%20Component%20Object%20Reference) (OtherBodyIndex :type Integer) (bFromSweep :type Boolean) (SweepResult :type Hit%20Result%20Structure%20%28by%20ref%29))
  (Utilities|Casting|CastToShapeshifter_original OtherActor)
  (bind _returnvalue (Actor|GetActorOfClass "/Game/GameContent/Assets/Door/BP_Door.BP_Door_C"))
  (Default|CollectedItem _returnvalue)
  (Actor|DestroyActor)
  (Audio|PlaySound2D "/Game/StarterContent/Audio/Explosion01.Explosion01" 1.0 1.0 0.0 0 0))

(event EventBeginPlay)

(fn ConstructionScript
  (Class|InterptoMovementComponent|AddControlPointPosition (Variables|Default|GetInterpToMovement) "0, 0, 0" true)
  (Class|InterptoMovementComponent|AddControlPointPosition (Variables|Default|GetInterpToMovement) (Variables|Default|GetPos) true))