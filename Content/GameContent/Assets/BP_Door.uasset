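; BP_Door is a door that swings open once enough items have been collected.
; Each CollectedItem call increments a counter, and on reaching MaxItems a DoOnce gate fires OpenDoor a single time and prints a notice.
; OpenDoor plays the DoorRotation timeline, which lerps the Door component's relative yaw to swing it open.
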(event Custom|Open%20Door
  (bind _door_rotation (Timeline|Door%20Rotation Play)
    (:Update
      (Transformation|SetRelativeRotation (Variables|Default|GetDoor) (Math|Rotator|MakeRotator 0.0 0.0 (Math|Float|Lerp 0.0 1.2e+02 _door_rotation)) false false))))

(event Custom|Collected%20Item
  (Math|Integer|IncrementInt (Variables|Default|GetCurrent%20Items)
    (:%20%20
      (if (>= (Variables|Default|GetCurrent%20Items) (Variables|Default|GetMaxItems))
        (Utilities|FlowControl|DoOnce false
          (:Completed
            (CallFunction|OpenDoor)
            (Development|PrintString "A Door Opened Somewhere")))))))

(fn ConstructionScript)